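; Room manager that assigns a random room type to each room in RoomsGrid when play begins.
; Each room draws its type from RoomTypes.RoomInstances through a random stream, then runs InitializeRoom.
; The stream is rebuilt per room from either the fixed Seed or a random integer, chosen by UseSeed.
; With UseSeed on, every room therefore draws from an identically seeded stream.
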(event `self.ReceiveBeginPlay`
  (for _array_element (`self.RoomsGrid`)
    (set `/Game/Blueprints/BP_Room.RoomType` (`KismetArrayLibrary.Array_RandomFromStream` (`/Game/Blueprints/PDA_RoomTypes.RoomInstances` (`self.RoomTypes`)) (`KismetMathLibrary.MakeRandomStream` (`KismetMathLibrary.SelectInt` (`self.Seed`) (`KismetMathLibrary.RandomInteger` 4096) (`self.UseSeed`)))) _array_element)
    (`/Game/Blueprints/BP_Room.InitializeRoom` _array_element)))

(fn `UserConstructionScript`)