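; BP_MainGameHUD is the HUD that draws the top-down player character's health bar on screen.
; BeginPlay caches the player as BP_TopDownCharacter, and every DrawHUD calls DrawHealth to render a label, black backing rectangle and fill.
; The backing scales with MaxHealth, while the fill shrinks with CurrentHealth and blends from green to red, using a safe divide and clamping at zero.
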(event `self.ReceiveBeginPlay`
  (set `self.PlayerRef` (cast `/Game/Blueprints/Characters/Player/BP_TopDownCharacter` (`GameplayStatics.GetPlayerCharacter` 0) :!pure true)))

(event `self.ReceiveDrawHUD`
  (params (SizeX :type Integer) (SizeY :type Integer))
  (`self.DrawHealth`))

(fn `DrawHealth`
  (bind _playerref (`self.PlayerRef`))
  (bind _maxhealth (`/Game/Blueprints/Characters/Player/BP_TopDownCharacter.MaxHealth` _playerref))
  (bind _returnvalue (`KismetMathLibrary.FMax` (`KismetMathLibrary.SafeDivide` (`/Game/Blueprints/Characters/Player/BP_TopDownCharacter.CurrentHealth` _playerref) _maxhealth)))
  (`self.DrawText` "Health:" (struct :`R` 0.1875 :`G` 0.1875 :`B` 0.1875 :`A` 1.0) 50.0 100.0 "/Engine/EngineFonts/Roboto.Roboto")
  (`self.DrawRect` (struct :`A` 1.0) 95.0 95.0 (+ (* _maxhealth 2.0) 10.0) 30.0)
  (`self.DrawRect` (make `LinearColor` (- 1.0 _returnvalue) _returnvalue 0.0 1.0) 100.0 100.0 (`KismetMathLibrary.FMax` (* _returnvalue (* _maxhealth 2.0))) 20.0))

(fn `UserConstructionScript`)